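; Prototype screen actor that shows a cargo manifest through its Widget component.
; On BeginPlay it casts the component's widget to CargoManifestWidget and passes it the TestManifest variable through SetCargoManifest.
; Overlap and Tick events are disabled stubs, and the construction script only calls its parent.
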(event `self.ReceiveBeginPlay`
  (`parent.ReceiveBeginPlay`)
  (bind _ascargo_manifest_widget (cast `CargoManifestWidget` (`WidgetComponent.GetWidget` (`self.Widget`))))
  (`CargoManifestWidget.SetCargoManifest` _ascargo_manifest_widget (`self.TestManifest`)))

(fn `UserConstructionScript`
  (`parent.UserConstructionScript`))